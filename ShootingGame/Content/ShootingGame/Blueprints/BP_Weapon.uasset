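; Data-driven gun actor for a networked shooter that attaches to a character's weapon socket and becomes a physics object when detached.
; WeaponData supplies mesh, montages, sound and muzzle effect; input plays montages, while notify events fire shots or refill ammo.
; Shots show effects client-side first, then the local player sends camera aim to ReqShoot for server ammo use, line trace and character damage.
; OnRep_Ammo updates the local HUD.
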(event `self.ReceiveBeginPlay`
  (bind (_weapondata_staticmesh _weapondata_shootmontage _weapondata_reloadmontage _weapondata_shootsound) (break `/Game/ShootingGame/Blueprints/ST_Weapon` (`self.WeaponData`)))
  (bind _weapondata_staticmesh_2 (break `/Game/ShootingGame/Blueprints/ST_Weapon` (`self.WeaponData`)))
  (`StaticMeshComponent.SetStaticMesh` (`self.StaticMesh`) _weapondata_staticmesh_2)
  (`AudioComponent.SetSound` (`self.Audio`) _weapondata_shootsound))

(event `self.PressReload`
  (bind (_weapondata_staticmesh _weapondata_shootmontage _weapondata_reloadmontage) (break `/Game/ShootingGame/Blueprints/ST_Weapon` (`self.WeaponData`)))
  (`Character.PlayAnimMontage` (`self.OwnCharacter`) _weapondata_reloadmontage 1.0 "None"))

(event `self.TriggerEvent`
  (params (IsPressed :type Boolean))
  (bind (_weapondata_staticmesh _weapondata_shootmontage) (break `/Game/ShootingGame/Blueprints/ST_Weapon` (`self.WeaponData`)))
  (if IsPressed
    (`Character.PlayAnimMontage` (`self.OwnCharacter`) _weapondata_shootmontage 1.0 "None")))

(event `self.NotifyShoot`
  (bind _returnvalue (`GameplayStatics.GetPlayerCameraManager` 0))
  ;[1 1 1] 클라이언트_선처리
  (bind _iscanuse (`self.IsCanUse`))
  (if _iscanuse
    (`self.ShowShootEffect`)
    ;[1 1 1] 데미지 요청 처리
    (if (== (`self.OwnCharacter`) (`GameplayStatics.GetPlayerCharacter` 0))
      (`self.ReqShoot` (`self.K2_GetActorLocation` _returnvalue) (`self.GetActorForwardVector` _returnvalue)))))

(event `ReqShoot`
  (params (StartPoint :type "Vector Structure") (ForwardVector :type "Vector Structure"))
  ;[1 1 1] 서버 처리
  (bind _iscanshoot (`self.UseAmmo`))
  (if _iscanshoot
    (`self.Process Server Shoot` StartPoint ForwardVector)))

(event `self.NotifyReload`
  ;[1 1 1] 장전시
  (`self.DoReload`))

(fn `AttachWeapon`
  (params (Character :type "Character Object Reference"))
  (returns (Result :type Boolean))
  (set `self.OwnCharacter` Character)
  (`PrimitiveComponent.SetSimulatePhysics` (`self.StaticMesh`) false)
  (`PrimitiveComponent.SetCollisionEnabled` (`self.StaticMesh`) "NoCollision")
  (`self.K2_AttachToComponent` (`Character.Mesh` Character) "weapon" "SnapToTarget" "SnapToTarget" "KeepWorld")
  (`self.Update Ammo To UI` (`self.Ammo`))
  (return false))

(fn `DetachWeapon`
  (returns (Result :type Boolean))
  (`self.Update Ammo To UI` 0)
  ;[1 1 1] 캐릭터 끊기
  (set `self.OwnCharacter` null)
  (`PrimitiveComponent.SetCollisionEnabled` (`self.StaticMesh`) "QueryAndPhysics")
  (`PrimitiveComponent.SetSimulatePhysics` (`self.StaticMesh`) true)
  (`SceneComponent.K2_DetachFromComponent` (`self.StaticMesh`) "KeepWorld" "KeepWorld" "KeepWorld" true)
  (return false))

(fn `DoReload`
  (bind (_weapondata_staticmesh _weapondata_shootmontage _weapondata_reloadmontage _weapondata_shootsound _weapondata_shooteffect _weapondata_maxammo) (break `/Game/ShootingGame/Blueprints/ST_Weapon` (`self.WeaponData`)))
  ;[1 1 1] 최대 장탄수 적용
  (set `self.Ammo` _weapondata_maxammo))

(fn `IsCanUse`
  (returns (IsCanUse :type Boolean))
  ;[1 1 1] 총알 남았는지 체크
  (return (> (`self.Ammo`) 0)))

(fn `OnRep_Ammo`
  (if (== (`Pawn.GetController` (`self.OwnCharacter`)) (`GameplayStatics.GetPlayerController` 0))
    (`self.Update Ammo To UI` (`self.Ammo`))))

(fn `Process Server Shoot`
  (params (StartPoint :type "Vector Structure") (ForwardVector :type "Vector Structure"))
  (bind _outhit (`KismetSystemLibrary.LineTraceSingleForObjects` (+ StartPoint (* ForwardVector 350.0)) (+ StartPoint (* ForwardVector (`self.Distance`))) (`|MakeArray` "ObjectTypeQuery3" "ObjectTypeQuery1" "ObjectTypeQuery2" "ObjectTypeQuery4" "ObjectTypeQuery5" "ObjectTypeQuery6" :!type "EObjectTypeQuery Enum") false (`|MakeArray` (`self.OwnCharacter`) :!type "Actor Object Reference") "Persistent"))
  (bind (_bblockinghit _binitialoverlap _time _distance _location _impactpoint _normal _impactnormal _physmat _hitactor) (`GameplayStatics.BreakHitResult` _outhit))
  (`KismetSystemLibrary.PrintString` (`KismetStringLibrary.Concat_StrStr` "HitActor - " (`KismetSystemLibrary.GetDisplayName` _hitactor)) true true (struct :`G` 0.66 :`B` 1.0 :`A` 1.0) 60.0)
  (bind _ascharacter (cast `Character` _hitactor))
  (`GameplayStatics.ApplyDamage` _ascharacter 10.0 (`Pawn.GetController` (`self.OwnCharacter`)) self))

(fn `ShowShootEffect`
  (bind (_weapondata_staticmesh _weapondata_shootmontage _weapondata_reloadmontage _weapondata_shootsound _weapondata_shooteffect) (break `/Game/ShootingGame/Blueprints/ST_Weapon` (`self.WeaponData`)))
  (bind (_returnvalue_location _returnvalue_rotation) (`KismetMathLibrary.BreakTransform` (`SceneComponent.GetSocketTransform` (`self.StaticMesh`) "Muzzle" "RTS_World")))
  (`GameplayStatics.SpawnEmitterAtLocation` _weapondata_shooteffect _returnvalue_location _returnvalue_rotation (0.3 0.3 0.3) true "AutoRelease")
  (`AudioComponent.Play` (`self.Audio`) 0.0))

(fn `Update Ammo To UI`
  (params (Ammo :type Integer))
  (bind _returnvalue (`GameplayStatics.GetPlayerController` 0))
  (bind _owncharacter (`self.OwnCharacter`))
  (`/Engine/EditorBlueprintResources/StandardMacros.IsValid` _owncharacter
    (:`Is Valid`
      (if (== (`Pawn.GetController` _owncharacter) _returnvalue)
        (bind _asshooting_hud (cast `/Game/ShootingGame/GameMode/ShootingHud` (`PlayerController.GetHUD` _returnvalue)))
        (`/Game/ShootingGame/Widget/HudWidget.SetAmmo` (`/Game/ShootingGame/GameMode/ShootingHud.HudWidget` _asshooting_hud) Ammo)))))

(fn `UseAmmo`
  (returns (IsCanShoot :type Boolean))
  (locals (CanUsed :type Boolean))
  (set `local.CanUsed` (> (`self.Ammo`) 0))
  (set `self.Ammo` (`KismetMathLibrary.Clamp` (- (`self.Ammo`) 1) 0 30))
  (return (`local.CanUsed`)))

(fn `UserConstructionScript`)