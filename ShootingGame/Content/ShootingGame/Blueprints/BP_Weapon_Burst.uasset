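; BP_Weapon_Burst is a weapon Blueprint for the shooting game that fires repeatedly while the trigger is held.
; TriggerEvent calls BurstShooting immediately on press and starts a looping short-interval timer by function name, then clears that timer on release, with no shot-count limit.
; BurstShooting only plays the shoot montage from WeaponData on the owning character, with no projectile or damage logic in this graph.
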(event `/Game/ShootingGame/Blueprints/BPI_Weapon.TriggerEvent`
  (params (IsPressed :type Boolean))
  (if IsPressed
    ;[1 1 1] 0.2초 기다림, 반복
    (`KismetSystemLibrary.K2_SetTimer` null "BurstShooting" 0.2 true)
    ;[1 1 1] 함수 실행
    (`self.BurstShooting`)
    (else
      ;[1 1 1] 취소
      (`KismetSystemLibrary.K2_ClearTimer` null "BurstShooting"))))

(fn `BurstShooting`
  (bind (_weapondata_staticmesh _weapondata_shootmontage) (break `/Game/ShootingGame/Blueprints/ST_Weapon` (`self.WeaponData`)))
  (`Character.PlayAnimMontage` (`self.OwnCharacter`) _weapondata_shootmontage 1.0 "None"))

(fn `UserConstructionScript`
  (`parent.UserConstructionScript`))